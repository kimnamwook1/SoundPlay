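; BP_BoxSpawner is a test-folder spawner that sends cubes with a given direction and color into one of twelve lanes.
; SpawnCube picks a child actor component from GetLanes by one-based lane number, casts its actor to BP_Lane and delegates the spawn.
; BeginPlay is empty, and a disconnected, delay-timed test chain is noted as a substitute for Level Sequence driving.
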(event EventBeginPlay)

(fn ConstructionScript)

(fn SpawnCube
  (params (Lane :type Integer) (Direction :type E_Direction%20Enum :default "NewEnumerator0") (Color :type E_Color%20Enum :default "NewEnumerator0"))
  (bind _asbp_lane (Utilities|Casting|CastToBP_Lane (Variables|/Script/Engine.ChildActorComponent|GetChildActor (Utilities|Array|Get(acopy) (CallFunction|GetLanes) (- Lane 1)))))
  (Default|SpawnCube _asbp_lane Direction Color))

(fn GetLanes
  (return (Utilities|Array|MakeArray (Variables|Default|GetLane1) (Variables|Default|GetLane2) (Variables|Default|GetLane3) (Variables|Default|GetLane4) (Variables|Default|GetLane5) (Variables|Default|GetLane6) (Variables|Default|GetLane7) (Variables|Default|GetLane8) (Variables|Default|GetLane9) (Variables|Default|GetLane10) (Variables|Default|GetLane11) (Variables|Default|GetLane12))))