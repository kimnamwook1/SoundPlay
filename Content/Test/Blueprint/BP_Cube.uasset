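; BP_Cube is a VR rhythm-style target cube that moves along negative X each tick, with a Color and a Direction marker.
; Construction builds a procedural box with collision, and Update refreshes marker visibility and material on BeginPlay and every tick.
; Overlap by the matching VRPawn hand (left blue, right red) triggers haptics, an explosion and destruction.
; A separate Slice event cuts the mesh by Direction, or a supplied normal for Punch, and launches it with physics.
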(event OnComponentHit(ProceduralMesh)
  (params (HitComponent :type Primitive%20Component%20Object%20Reference) (OtherActor :type Actor%20Object%20Reference) (OtherComp :type Primitive%20Component%20Object%20Reference) (NormalImpulse :type Vector :default "0, 0, 0") (Hit :type Hit%20Result%20Structure%20%28by%20ref%29)))

(event OnComponentBeginOverlap(ProceduralMesh)
  (params (OverlappedComponent :type Primitive%20Component%20Object%20Reference) (OtherActor :type Actor%20Object%20Reference) (OtherComp :type Primitive%20Component%20Object%20Reference) (OtherBodyIndex :type Integer) (bFromSweep :type Boolean) (SweepResult :type Hit%20Result%20Structure%20%28by%20ref%29))
  ;[1 1 1] When Overlapped
  (bind _asvrpawn (Utilities|Casting|CastToVRPawn OtherActor))
  (if (and (== (Variables|/Game/VRTemplate/Blueprints/VRPawn.VRPawn_C|GetLeftHand _asvrpawn) OtherComp) (Utilities|Enum|Equal(Enum) (Variables|Default|GetColor) "NewEnumerator1"))
    (Class|PlayerController|PlayHapticEffect (Game|GetPlayerController 0) "/Game/VRTemplate/Haptics/PistolFireHapticEffect.PistolFireHapticEffect" "Left" 1.0 false)
    (Effects|SpawnEmitteratLocation "/Game/StarterContent/Particles/P_Explosion.P_Explosion" (Transformation|GetActorLocation) "0, 0, 0" "0.200000,0.200000,0.200000")
    (Actor|DestroyActor)
    (elif (and (== (Variables|/Game/VRTemplate/Blueprints/VRPawn.VRPawn_C|GetRightHand _asvrpawn) OtherComp) (Utilities|Enum|Equal(Enum) (Variables|Default|GetColor) "NewEnumerator0"))
      (Class|PlayerController|PlayHapticEffect (Game|GetPlayerController 0) "/Game/VRTemplate/Haptics/PistolFireHapticEffect.PistolFireHapticEffect" "Right" 1.0 false)
      (Effects|SpawnEmitteratLocation "/Game/StarterContent/Particles/P_Explosion.P_Explosion" (Transformation|GetActorLocation) "0, 0, 0" "0.200000,0.200000,0.200000")
      (Actor|DestroyActor))))

(event Custom|Slice
  (params (CutNormalVector :type Vector))
  (bind _outotherhalfprocmesh (Class|KismetProceduralMeshLibrary|SliceProceduralMesh (Variables|Default|GetProceduralMesh) (Transformation|GetActorLocation) (Utilities|Select :Index (Variables|Default|GetDirection) :NewEnumerator0 "0,1.000000, 0" :NewEnumerator1 "0,-1.000000, 0" :NewEnumerator2 "0, 0,1.000000" :NewEnumerator3 "0, 0,-1.000000" :NewEnumerator4 CutNormalVector) true "CreateNewSectionForCap"))
  (Physics|SetSimulatePhysics _outotherhalfprocmesh true)
  (Physics|AddImpulse _outotherhalfprocmesh "500.000000, 0,350.000000" "None" true)
  (for _array_element (Utilities|Array|MakeArray (Variables|Default|GetLeft) (Variables|Default|GetRight) (Variables|Default|GetPunch) (Variables|Default|GetUp) (Variables|Default|GetDown))
    (Components|DestroyComponent _array_element)))

(event EventTick
  (params (DeltaSeconds :type Float%20%28single-precision%29))
  (bind _returnvalue (Transformation|GetActorLocation))
  ;[1 1 1] Move Cube by Tick
  (Transformation|SetActorLocation (Math|Vector|MakeVector (+ (.x _returnvalue) -1e+01) (.y _returnvalue) (.z _returnvalue)) false false)
  (CallFunction|Update))

(event EventBeginPlay
  (CallFunction|Update))

(fn ConstructionScript
  (bind (_vertices _triangles _normals _uvs _tangents) (Class|KismetProceduralMeshLibrary|GenerateBoxMesh "45.000000,45.000000,45.000000"))
  (Class|ProceduralMeshComponent|CreateMeshSectionLinearColor (Variables|Default|GetProceduralMesh) 0 _vertices _triangles _normals 0 0 0 0 0 _tangents true)
  (Class|ProceduralMeshComponent|AddCollisionConvexMesh (Variables|Default|GetProceduralMesh) _vertices))

(fn Update
  (bind _direction (Variables|Default|GetDirection))
  (bind _left (Variables|Default|GetLeft))
  (bind _punch (Variables|Default|GetPunch))
  (bind _up (Variables|Default|GetUp))
  (bind _down (Variables|Default|GetDown))
  (bind _right (Variables|Default|GetRight))
  (bind _returnvalue (Utilities|Select :Index _direction :NewEnumerator0 _up :NewEnumerator1 _down :NewEnumerator2 _left :NewEnumerator3 _right :NewEnumerator4 _punch))
  (Rendering|SetVisibility _returnvalue true false)
  (Variables|Default|SetChosenCube _returnvalue)
  (for _array_element (Utilities|Array|MakeArray (Variables|Default|GetUp) (Variables|Default|GetDown) (Variables|Default|GetRight) (Variables|Default|GetLeft) (Variables|Default|GetPunch))
    (Rendering|SetVisibility _array_element (== _array_element (Variables|Default|GetChosenCube)) false))
  (Rendering|Material|SetMaterial (Variables|Default|GetProceduralMesh) 0 (Utilities|Select :Index (Variables|Default|GetColor) :NewEnumerator0 "/Game/Test/Material/MI_CubeColor_Red.MI_CubeColor_Red" :NewEnumerator1 "/Game/Test/Material/MI_CubeColor_Blue.MI_CubeColor_Blue")))